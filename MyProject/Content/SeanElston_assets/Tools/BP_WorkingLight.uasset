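; BP_WorkingLight is a placeable light tool Blueprint that wraps a point light with exposed settings for level lighting.
; Its construction script pushes radius, intensity, volumetric scattering, temperature and color onto the PointLight component.
; Each numeric setting is clamped to a fixed range before being applied.
; The event graph holds only disabled default events, so nothing runs at play time.
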(event EventBeginPlay)

(event Collision|EventActorBeginOverlap
  (params (OtherActor :type Actor%20Object%20Reference)))

(event EventTick
  (params (DeltaSeconds :type Float%20%28single-precision%29)))

(fn ConstructionScript
  (bind _pointlight (Variables|Default|GetPointLight))
  (Utilities|FlowControl|Sequence
    (:then_0
      ;[0.15 0.15 0.15 0.5] Radius
      (Rendering|Lighting|SetAttenuationRadius _pointlight (Math|Float|Clamp(Float) (Variables|LightingTool|GetRadius) 0.0 2.5e+03)))
    (:then_1
      ;[0.15 0.15 0.15 0.5] Intensity
      (Rendering|Components|Light|SetIntensity _pointlight (Math|Float|Clamp(Float) (Variables|LightingTool|GetIntensity) 0.0 8e+02)))
    (:then_2
      ;[0.15 0.15 0.15 0.5] Volumetric Scattering
      (Class|LightComponent|SetVolumetricScatteringIntensity _pointlight (Math|Float|Clamp(Float) (Variables|LightingTool|GetVolumetric%20Intensity) 0.0 1e+01)))
    (:then_3
      ;[0.15 0.15 0.15 0.5] Temp
      (Class|LightComponent|SetTemperature _pointlight (Math|Float|Clamp(Float) (Variables|LightingTool|GetTemp) 0.0 1.2e+04)))
    (:then_4
      (Rendering|Components|Light|SetLightColor _pointlight (Math|Conversions|ToLinearColor(Color) (Variables|LightingTool|GetColor)) true))))